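; BP_XRCharacter is a character Blueprint that colors its health bar according to whether the character is an attacker or a defender.
; On BeginPlay it casts the HealthWidgetComponent's widget to WBP_HealthBar, caches it, then applies the color if the reference is valid.
; DecideHealthColor maps ObjectType to the offence or defence color variable.
; Tick, overlap and the construction script are empty.
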(event `self.ReceiveBeginPlay`
  (bind _health_barwidget (`self.Health BarWidget`))
  (`|ExecutionSequence`
    (:`then_0`
      (bind _aswbp_health_bar (cast `/Game/Blueprints/UI/WBP_HealthBar` (`WidgetComponent.GetUserWidgetObject` (`self.HealthWidgetComponent`))))
      (set `self.Health BarWidget` _aswbp_health_bar))
    (:`then_1`
      (`/Engine/EditorBlueprintResources/StandardMacros.IsValid` _health_barwidget
        (:`Is Valid`
          (bind _selectedcolor (`self.DecideHealthColor`))
          (`/Game/Blueprints/UI/WBP_HealthBar.Set Health Color` _health_barwidget _selectedcolor))))))

(fn `DecideHealthColor`
  (returns (SelectedColor :type "LinearColor Structure"))
  (locals (Color :type "LinearColor Structure"))
  (switch `EObjectType` (`self.objectType`)
    (:`EOT_ATTACKER`
      (set `local.Color` (`self.OffenceColor`)))
    (:`EOT_DEFENDER`
      (set `local.Color` (`self.DeffenceColor`))))
  (return (`local.Color`)))

(fn `UserConstructionScript`)